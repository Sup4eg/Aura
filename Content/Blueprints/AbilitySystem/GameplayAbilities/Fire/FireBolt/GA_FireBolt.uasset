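; Gameplay ability that casts a Fire Bolt projectile toward the location under the mouse.
; A target-data task supplies the hit location, and the avatar is turned toward it through CombatInterface.
; The cast montage then plays while a gameplay event task waits for the montage's FireBolt tag, which triggers SpawnProjectile at that location.
; The graph never calls EndAbility.
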(event Ability|EventActivateAbility
  (bind _returnvalue (Ability|GetAvatarActorfromActorInfo))
  (bind _data (|TargetDataUnderMouse)
    (:ValidData
      (bind _output_get (Variables|Default|SetProjectileTargetLocation (.location (Ability|TargetData|GetHitResultfromTargetData _data))))
      (if (Utilities|DoesObjectImplementInterface _returnvalue "/Script/Aura.CombatInterface")
        (Class|CombatInterface|SetFacingTarget(Message) _returnvalue _output_get)
        (|PlayMontageandWaitProxy "None" "/Game/Assets/Characters/Aura/Animations/Abilities/AM_CastFireBolt.AM_CastFireBolt" 1.0 "None" true 1.0 0.0 false
          (:then
            (Ability|Tasks|WaitGameplayEvent "(TagName=\"Event.Montage.FireBolt\")" 0
              (:EventReceived
                (Class|AuraProjectileSpell|SpawnProjectile (Variables|Default|GetProjectileTargetLocation))))))))))

(event Ability|EventOnEndAbility
  (params (bWasCancelled :type Boolean)))